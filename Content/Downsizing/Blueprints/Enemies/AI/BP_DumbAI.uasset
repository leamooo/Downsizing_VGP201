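; BP_DumbAI is a simple melee enemy that stays still until it spots the player, then chases and damages them.
; Pawn sensing sets a never-cleared seen flag and starts AI Move To, applying damage on arrival; each sighting re-arms the attack.
; Incoming damage lowers clamped health and updates a widget health bar.
; At zero health, it increments the player HUD's score and destroys itself.
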(event `self.ReceiveBeginPlay`
  (`self.UpdateEnemyHealthBar`))

(event `self.ReceiveTick`
  (params (DeltaSeconds :type "Float (single-precision)"))
  (if (not (`self.IsSeeingPlayer?`))
    (`MovementComponent.StopMovementImmediately` (`self.CharacterMovement`))))

(event `self.PawnSensing.OnSeePawn`
  (params (Pawn :type "Pawn Object Reference"))
  (set `self.IsSeeingPlayer?` true)
  (`self.FollowPlayer`))

(event `FollowPlayer`
  (bind _returnvalue (`GameplayStatics.GetPlayerCharacter` 0))
  (set `self.CanAttack?` true)
  (if (`self.IsSeeingPlayer?`)
    (`|AIMoveTo` self (0.0 0.0 0.0) _returnvalue 50.0
      (:`OnSuccess`
        (if (`self.CanAttack?`)
          (set `self.CanAttack?` false)
          (`KismetSystemLibrary.PrintString` "Enemy Attacked WHACK!")
          (`GameplayStatics.ApplyDamage` _returnvalue (`self.Damage Amt`))
          (`KismetSystemLibrary.Delay` 3.0))))))

(event `self.ReceiveAnyDamage`
  (params (Damage :type "Float (single-precision)") (DamageType :type "DamageType Object Reference") (InstigatedBy :type "Controller Object Reference") (DamageCauser :type "Actor Object Reference"))
  ;[1 1 1] Damage Taking
  (if (not (`self.IsEnemyDead?`))
    (bind _output_get (set `self.EnemyHealth` (`KismetMathLibrary.FClamp` (- (`self.EnemyHealth`) Damage) 0.0 (`self.EnemyMaxHealth`))))
    (`self.UpdateEnemyHealthBar`)
    (if (== 0.0 _output_get)
      (bind _asbp_player (cast `/Game/Downsizing/Blueprints/Player/BP_Player` (`GameplayStatics.GetPlayerCharacter` 0)))
      (bind _wbp_gamehud (`/Game/Downsizing/Blueprints/Player/BP_Player.WBP_GameHUD` _asbp_player))
      (bind _score (`/Game/Downsizing/Blueprints/GUI/WBP_GameHUD.Score` _wbp_gamehud))
      (bind _result (`/Engine/EditorBlueprintResources/StandardMacros.IncrementInt` _score)
        (:`  `
          (`/Game/Downsizing/Blueprints/GUI/WBP_GameHUD.SetScore` _wbp_gamehud _result)
          (`self.K2_DestroyActor`)
          (`KismetSystemLibrary.PrintString` (`KismetStringLibrary.Conv_IntToString` _score)))))))

(fn `UpdateEnemyHealthBar`
  (bind _enemyhealth (`self.EnemyHealth`))
  (bind _aswbp_enemy_health_bar (cast `/Game/Downsizing/Blueprints/GUI/EnemyGUI/WBP_EnemyHealthBar` (`WidgetComponent.GetUserWidgetObject` (`self.HealthBar`))))
  (`/Engine/EditorBlueprintResources/StandardMacros.IsValid` _aswbp_enemy_health_bar
    (:`Is Valid`
      (`ProgressBar.SetPercent` (`/Game/Downsizing/Blueprints/GUI/EnemyGUI/WBP_EnemyHealthBar.EnemyHealthbar` _aswbp_enemy_health_bar) (/ _enemyhealth (`self.EnemyMaxHealth`)))
      (`KismetSystemLibrary.PrintString` (`KismetStringLibrary.Conv_DoubleToString` _enemyhealth))
      (return))))

(fn `UserConstructionScript`)