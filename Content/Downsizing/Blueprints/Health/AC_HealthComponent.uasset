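; Actor component that stores health for its owner and exposes heal, damage, death-check and normalized-health functions.
; BeginPlay calls Init to set the min and max bounds and fill health to max.
; All changes pass through SetHealth, which clamps to those bounds.
; Damage subtracts current health from the damage amount rather than the reverse, and HealFull prints a debug message.
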(event `self.ReceiveBeginPlay`
  (`self.Init` (`self.MinHealth`) (`self.MaxHealth`)))

(fn `ClampHealth`
  (params (Value :type "Float (double-precision)"))
  (returns (ReturnValue :type "Float (double-precision)"))
  (return (`KismetMathLibrary.FClamp` Value (`self.MinHealth`) (`self.MaxHealth`))))

(fn `Damage`
  (params (DamageAmount :type "Float (double-precision)"))
  (`self.SetHealth` (`self.ClampHealth` (- DamageAmount (`self.GetHealth`)))))

(fn `GetHealth`
  (returns (Value :type "Float (double-precision)"))
  (return (`self.Health`)))

(fn `GetNormalizedHealth`
  (returns (Value :type "Float (double-precision)"))
  (return (`KismetMathLibrary.FClamp` (/ (`self.Health`) (`self.MaxHealth`)) 0.0 1.0)))

(fn `Heal`
  (params (HealAmt :type "Float (double-precision)"))
  (`self.SetHealth` (`self.ClampHealth` (+ HealAmt (`self.GetHealth`)))))

(fn `HealFull`
  (`self.Heal` (`self.MaxHealth`))
  (`KismetSystemLibrary.PrintString` "Player Has Been heaed to full"))

(fn `Init`
  (params (MinHealth :type "Float (double-precision)") (MaxHealth :type "Float (double-precision)"))
  (set `self.MinHealth` MinHealth)
  (bind _output_get (set `self.MaxHealth` MaxHealth))
  (`self.SetHealth` _output_get))

(fn `IsDead`
  (returns (Value :type Boolean))
  (return (<= (`self.GetHealth`) 0.0)))

(fn `SetHealth`
  (params (NewHealth :type "Float (double-precision)"))
  (set `self.Health` (`self.ClampHealth` NewHealth)))