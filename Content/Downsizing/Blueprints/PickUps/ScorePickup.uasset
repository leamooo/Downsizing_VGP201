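; ScorePickup is a pickup Blueprint that adds one to the player's score and destroys itself when its box is overlapped.
; The overlap event casts the local player character to BP_Player, increments Score on its game HUD widget, passes it to SetScore, and prints it.
; The overlapping actor is never checked, as the Player tag test is left unconnected, so any overlap can award the point.
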(event `self.Box.OnComponentBeginOverlap`
  (params (OverlappedComponent :type "PrimitiveComponent Object Reference") (OtherActor :type "Actor Object Reference") (OtherComp :type "PrimitiveComponent Object Reference") (OtherBodyIndex :type Integer) (bFromSweep :type Boolean) (SweepResult :type "HitResult Structure (by ref)"))
  (bind _asbp_player (cast `/Game/Downsizing/Blueprints/Player/BP_Player` (`GameplayStatics.GetPlayerCharacter` 0)))
  (bind _score (`/Game/Downsizing/Blueprints/GUI/WBP_GameHUD.Score` (`/Game/Downsizing/Blueprints/Player/BP_Player.WBP_GameHUD` _asbp_player)))
  (bind _result (`/Engine/EditorBlueprintResources/StandardMacros.IncrementInt` _score)
    (:`  `
      (`/Game/Downsizing/Blueprints/GUI/WBP_GameHUD.SetScore` (`/Game/Downsizing/Blueprints/Player/BP_Player.WBP_GameHUD` _asbp_player) _result)
      (`self.K2_DestroyActor`)
      (`KismetSystemLibrary.PrintString` (`KismetStringLibrary.Conv_IntToString` _score)))))

(fn `UserConstructionScript`)